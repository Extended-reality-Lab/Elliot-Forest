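; CameraSpeed is a debug-style Blueprint that adjusts the player pawn's movement speed at runtime from the keyboard.
; The Add and Subtract keys cast player pawn 0's movement component to FloatingPawnMovement, then raise or lower its MaxSpeed by a fixed step.
; Each press prints the new speed, and no limit is applied to the value.
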(event `Key|Add`
  (params (Key :type "Key Structure"))
  (:`Pressed`
    (bind _asfloating_pawn_movement (cast `FloatingPawnMovement` (`Pawn.GetMovementComponent` (`GameplayStatics.GetPlayerPawn` 0))))
    (bind _output_get (set `FloatingPawnMovement.MaxSpeed` (+ (`MovementComponent.GetMaxSpeed` _asfloating_pawn_movement) 100.0) _asfloating_pawn_movement))
    (`KismetSystemLibrary.PrintString` (`KismetStringLibrary.Conv_DoubleToString` _output_get))))

(event `self.ReceiveBeginPlay`)

(event `Key|Subtract`
  (params (Key :type "Key Structure"))
  (:`Pressed`
    (bind _asfloating_pawn_movement (cast `FloatingPawnMovement` (`Pawn.GetMovementComponent` (`GameplayStatics.GetPlayerPawn` 0))))
    (bind _output_get (set `FloatingPawnMovement.MaxSpeed` (- (`MovementComponent.GetMaxSpeed` _asfloating_pawn_movement) 100.0) _asfloating_pawn_movement))
    (`KismetSystemLibrary.PrintString` (`KismetStringLibrary.Conv_DoubleToString` _output_get))))

(fn `UserConstructionScript`)