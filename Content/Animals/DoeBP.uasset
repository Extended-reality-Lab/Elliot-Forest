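; Doe animal actor that travels along its Spline component, starting at BeginPlay.
; MoveAnimal scales a timeline's play rate by spline length for consistent speed, then places the skeletal mesh at constant-velocity spline transforms with a yaw correction.
; SnapToTerrain traces up, then down, to move spline points onto the Landscape, but its call here is disconnected.
; AI movement and AnimalPath lookup logic are also left unconnected.
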(event `self.ReceiveBeginPlay`
  (`self.MoveAnimal`))

(event `MoveAnimal`
  (bind _spline (`self.Spline`))
  (`TimelineComponent.SetPlayRate` (`self.MoveAnimalT`) (/ 1.0 (/ (`SplineComponent.GetSplineLength` _spline) 1500.0)))
  (bind (_direction _movetrack) (`Timeline|MoveAnimalT`)
    (:`Update`
      (bind (_returnvalue_location _returnvalue_rotation) (`KismetMathLibrary.BreakTransform` (`SplineComponent.GetTransformAtTime` _spline _movetrack "World" true false)))
      (`SceneComponent.K2_SetWorldLocationAndRotation` (`self.SkeletalMesh`) _returnvalue_location (`KismetMathLibrary.ComposeRotators` _returnvalue_rotation (struct :`Yaw` -90.0)) false false))))

(fn `SnapToTerrain`
  (locals (`Found Above` :type Boolean))
  (bind _spline (`self.Spline`))
  (for _index (range (`SplineComponent.GetNumberOfSplinePoints` _spline))
    (set `local.Found Above` false)
    (bind _returnvalue (`SplineComponent.GetLocationAtSplinePoint` _spline _index "World"))
    (bind _outhits (`KismetSystemLibrary.LineTraceMulti` _returnvalue (+ _returnvalue (0.0 0.0 100000.0)) "TraceTypeQuery1"))
    (for _array_element _outhits
      (cast `Landscape` (`.HitActor` (`GameplayStatics.BreakHitResult` _array_element)))
      (set `local.Found Above` true)
      (`SplineComponent.SetLocationAtSplinePoint` (`self.Spline`) _index (`.ImpactPoint` (`GameplayStatics.BreakHitResult` _array_element)) "World" true))
    (if (not (`local.Found Above`))
      (bind _returnvalue_2 (`SplineComponent.GetLocationAtSplinePoint` (`self.Spline`) _index "World"))
      (bind _outhits_2 (`KismetSystemLibrary.LineTraceMulti` _returnvalue_2 (+ _returnvalue_2 (0.0 0.0 -100000.0)) "TraceTypeQuery1"))
      (for _array_element_2 _outhits_2
        (cast `Landscape` (`.HitActor` (`GameplayStatics.BreakHitResult` _array_element_2)))
        (`SplineComponent.SetLocationAtSplinePoint` (`self.Spline`) _index (`.ImpactPoint` (`GameplayStatics.BreakHitResult` _array_element_2)) "World" true)))))

(fn `UserConstructionScript`)