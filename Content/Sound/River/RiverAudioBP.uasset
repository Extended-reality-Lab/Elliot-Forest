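; River audio Blueprint that keeps a single river sound at the point on the water splines closest to the player.
; On BeginPlay it finds a WaterSpline actor, has it generate splines if empty, then starts TrackPlayer, which repeats every second.
; Each pass moves RiverSound just above the nearest spline point and starts playback within range, never stopping it.
; SnapToTerrain holds only disconnected landscape-trace logic.
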(event `self.ReceiveBeginPlay`
  (bind _returnvalue (`GameplayStatics.GetPlayerPawn` 0))
  ;[1 1 1] Validate Player and Get Water Spline Actor
  (`/Engine/EditorBlueprintResources/StandardMacros.IsValid` _returnvalue
    (:`Is Valid`
      (set `self.Player` _returnvalue)
      (bind _returnvalue_2 (`GameplayStatics.GetActorOfClass` "/Game/Blueprints/WaterSpline.WaterSpline_C"))
      (bind _output_get (set `self.rivers` _returnvalue_2))
      ;[1 1 1] Check if Spline Has Points
      (if (== (`KismetArrayLibrary.Array_Length` (`/Game/Blueprints/WaterSpline.splines` _output_get)) 0)
        ;[1 1 1] Generate Spline If No Points
        (`/Game/Blueprints/WaterSpline.GenerateSpline` _output_get))
      (`self.TrackPlayer`))))

(event `TrackPlayer`
  (bind _riversound (`self.RiverSound`))
  (bind _returnvalue (`self.K2_GetActorLocation` (`self.Player`)))
  (set `self.MinWaterDistance` 10000000.0)
  ;[1 1 1] Loop Through Spline Points
  (for _array_element (`/Game/Blueprints/WaterSpline.splines` (`self.rivers`))
    (bind _returnvalue_2 (`SplineComponent.FindLocationClosestToWorldLocation` _array_element _returnvalue "World"))
    (bind _returnvalue_3 (`KismetMathLibrary.Vector_Distance` _returnvalue_2 _returnvalue))
    ;[1 1 1] Check if distance between spline points and player is smaller than a before
    (if (< _returnvalue_3 (`self.MinWaterDistance`))
      (bind _output_get (set `self.MinWaterDistance` _returnvalue_3))
      (bind (_x _y _z) (`KismetMathLibrary.BreakVector3f` _returnvalue_2))
      ;[1 1 1] Set Sound Location and Play  if Player is Within a Set Distance
      (`SceneComponent.K2_SetWorldLocation` _riversound (`KismetMathLibrary.MakeVector` _x _y (+ _z 50.0)) false false)
      (if (and (not (`AudioComponent.IsPlaying` _riversound)) (<= _output_get 8000.0))
        (`AudioComponent.Play` _riversound 0.0))))
  (`KismetSystemLibrary.Delay` 1.0)
  (`self.TrackPlayer`))

(fn `SnapToTerrain`
  (locals (FoundAbove :type Boolean)))

(fn `UserConstructionScript`)