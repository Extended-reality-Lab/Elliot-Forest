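; WaterSpline actor that builds water stream splines from Data Table rows, generating on BeginPlay if the first WaterSpline found has none.
; GenerateSpline clears old splines, starts a new one whenever REACHID changes so streams stay separate, and georeferences projected coordinates into points.
; SplineSnap traces up, then down, to move points onto the Landscape, but its call and the spline-mesh building sit in unconnected logic that never runs.
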(event `self.ReceiveBeginPlay`
  (bind _outactors (`GameplayStatics.GetAllActorsOfClass` "WaterSpline_C"))
  (if (== (`KismetArrayLibrary.Array_Length` _outactors) 0)
    (`self.GenerateSpline`)
    (elif (== (`KismetArrayLibrary.Array_Length` (`/Game/Blueprints/WaterSpline.splines` (`|GetArrayItem` _outactors))) 0)
      (`self.GenerateSpline`))))

(fn `GenerateSpline`
  (locals (CurrentReach :type "Float (double-precision)" :default -1.0))
  (bind _splines (`self.splines`))
  (bind _splines_2 (`self.splines`))
  (bind _splines_3 (`self.splines`))
  ;[1 1 1] Remove the components and the references
  (for _array_element _splines
    (`ActorComponent.K2_DestroyComponent` _array_element))
  (`KismetArrayLibrary.Array_Clear` _splines)
  ;[1 1 1] Get Data From CSV File
  (bind _outrownames (`DataTableFunctionLibrary.GetDataTableRowNames` (`self.Table`)))
  (for _index (range (+ (`KismetArrayLibrary.Array_LastIndex` _outrownames) 1))
    (bind _returnvalue (`|GetDataTableRow` (`self.Table`) (`|GetArrayItem` _outrownames _index))
      (:`then`
        (bind (_z _orig_fid _reach_id _fish _miles _meters _mrw_crw _p_class _zone _shape_leng _shape_length _point_x _point_y _xcoord _ycoord) (break `/Game/Blueprints/WaterData` _returnvalue))
        ;[1 1 1] Check If Next Point is Apart of New Stream, So We Dont add a Spline Point Across Land
        (if (not (== (`local.CurrentReach`) _reach_id))
          (set `local.CurrentReach` _reach_id)
          (bind _returnvalue_2 (`AddComponent|NODE_AddSplineComponent-0`))
          (`KismetArrayLibrary.Array_Add` _splines_3 _returnvalue_2)
          (`SplineComponent.ClearSplinePoints` _returnvalue_2 false))
        ;[1 1 1] Georeference and Add Spline Point
        (bind _enginecoordinates (`GeoReferencingSystem.K2_ProjectedToEngine` (`GeoReferencingSystem.GetGeoReferencingSystem`) (`KismetMathLibrary.MakeVector` _xcoord _ycoord _z)))
        (`SplineComponent.AddSplinePoint` (`|GetArrayItem` _splines_3 (`KismetArrayLibrary.Array_LastIndex` _splines_3)) _enginecoordinates "World" false))))
  (`SplineComponent.UpdateSpline` (`|GetArrayItem` _splines_2 (`KismetArrayLibrary.Array_LastIndex` _splines_2))))

(fn `SplineSnap`
  (params (NewParam :type "SplineComponent Object Reference"))
  ;[1 1 1] Loop Through Number of Spline Points
  (for _index (range (`SplineComponent.GetNumberOfSplinePoints` NewParam))
    (set `self.FoundAbove` false)
    (bind _returnvalue (`SplineComponent.GetLocationAtSplinePoint` NewParam _index "World"))
    (bind _outhits (`KismetSystemLibrary.LineTraceMulti` _returnvalue (+ _returnvalue (0.0 0.0 100000.0)) "TraceTypeQuery1"))
    (for _array_element _outhits
      ;[1 1 1] Check To See if Spline Point is Above Landscape
      (cast `Landscape` (`.HitActor` (`GameplayStatics.BreakHitResult` _array_element)))
      (set `self.FoundAbove` true)
      (`SplineComponent.SetLocationAtSplinePoint` NewParam _index (`.ImpactPoint` (`GameplayStatics.BreakHitResult` _array_element)) "World" true))
    ;[1 1 1] If Spline Point Was Found Above, Move it to the Landscape
    (if (not (`self.FoundAbove`))
      (bind _returnvalue_2 (`SplineComponent.GetLocationAtSplinePoint` NewParam _index "World"))
      (bind _outhits_2 (`KismetSystemLibrary.LineTraceMulti` _returnvalue_2 (+ _returnvalue_2 (0.0 0.0 -100000.0)) "TraceTypeQuery1"))
      (for _array_element_2 _outhits_2
        (cast `Landscape` (`.HitActor` (`GameplayStatics.BreakHitResult` _array_element_2)))
        (`SplineComponent.SetLocationAtSplinePoint` NewParam _index (`.ImpactPoint` (`GameplayStatics.BreakHitResult` _array_element_2)) "World" true)))))

(fn `UserConstructionScript`)