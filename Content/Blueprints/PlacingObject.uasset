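; Actor that populates the level with georeferenced trees from a data table on BeginPlay.
; PlaceTrees replaces its hierarchical instanced static mesh components with a new one, converting each row's projected coordinates to engine space through the GeoReferencing system.
; Instances get random yaw and slight tilt, with height scaled from feet against mesh bounds.
; Width follows either that height scale or the square root of canopy area, depending on UniformScale.
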(event `self.ReceiveBeginPlay`
  (`self.PlaceTrees`))

(fn `PlaceTrees`
  (bind _table (`self.Table`))
  (bind (_min _max) (break `Box` (`StaticMesh.GetBoundingBox` (`self.Mesh`))))
  (for _array_element (`self.K2_GetComponentsByClass` "/Script/Engine.HierarchicalInstancedStaticMeshComponent")
    (`ActorComponent.K2_DestroyComponent` _array_element))
  (bind _returnvalue (`AddComponent|NODE_AddHierarchicalInstancedStaticMeshComponent-1`))
  (bind _output_get (set `self.ISM` _returnvalue))
  (`StaticMeshComponent.SetStaticMesh` _output_get (`self.Mesh`))
  (bind _outrownames (`DataTableFunctionLibrary.GetDataTableRowNames` _table))
  (for _array_element_2 _outrownames
    (bind _returnvalue_2 (`|GetDataTableRow` _table _array_element_2)
      (:`then`
        (bind (_xcoord _ycoord _species _z _ht _canopyarea) (break `/Game/Blueprints/TreeData` _returnvalue_2))
        (bind _output_get_2 (set `self.XCoord` _xcoord))
        (bind _output_get_3 (set `self.YCoord` _ycoord))
        (bind _output_get_4 (set `self.Z` _z))
        (bind _enginecoordinates (`GeoReferencingSystem.K2_ProjectedToEngine` (`GeoReferencingSystem.GetGeoReferencingSystem`) (`KismetMathLibrary.MakeVector` _output_get_2 _output_get_3 _output_get_4)))
        (bind _returnvalue_3 (/ (* _ht 30.48) (.z (- _max _min))))
        (bind _returnvalue_4 (select `bool` (`self.UniformScale`) :`false` (/ (* (`KismetMathLibrary.Sqrt` _canopyarea) 30.48) (`KismetMathLibrary.FMax` (.x (- _max _min)) (.y (- _max _min)))) :`true` _returnvalue_3))
        (`InstancedStaticMeshComponent.AddInstance` (`self.ISM`) (`KismetMathLibrary.MakeTransform` _enginecoordinates (`KismetMathLibrary.MakeRotator` (`KismetMathLibrary.RandomFloatInRange` 0.0 7.0) (`KismetMathLibrary.RandomFloatInRange` 0.0 7.0) (`KismetMathLibrary.RandomFloatInRange` 0.0 360.0)) (`KismetMathLibrary.MakeVector` _returnvalue_4 _returnvalue_4 _returnvalue_3)) true))))
  (return))

(fn `UserConstructionScript`)