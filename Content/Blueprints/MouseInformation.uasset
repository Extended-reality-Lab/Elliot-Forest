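; Shows a floating info card with species, height and diameter when the player Shift+left-clicks a tree.
; Holding Shift shows the cursor, and a click traces WorldDynamic objects under it.
; Cast2Tree reads the hit instance's data from TreeManagerThinning or TreeManager, returning an empty species otherwise to hide the card.
; The TreeInfo widget is placed just off the impact point, facing back along the trace, with clamped distance-based scale.
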(event `self.ReceiveBeginPlay`
  (bind _infocard (`self.InfoCard`))
  ;[1 1 1] Create UI Element and Set to Not Visible
  (bind _returnvalue (`|CreateWidget` "/Game/Widgets/TreeInfo.TreeInfo_C"))
  (`WidgetComponent.SetWidget` _infocard _returnvalue)
  (set `Widget.Visibility` "Collapsed" (`WidgetComponent.GetWidget` _infocard)))

(event `Key|Shift+LeftMouseButton`
  (params (Key :type "Key Structure"))
  (bind _infocard (`self.InfoCard`))
  (bind _infocard_2 (`self.InfoCard`))
  (bind _hitresult (`PlayerController.GetHitResultUnderCursorForObjects` (`GameplayStatics.GetPlayerController` 0) (`|MakeArray` "ObjectTypeQuery2" :!type "EObjectTypeQuery Enum") true))
  (bind (_bblockinghit _binitialoverlap _time _distance _location _impactpoint _normal _impactnormal _physmat _hitactor _hitcomponent _hitbonename _bonename _hititem _elementindex _faceindex _tracestart _traceend) (`GameplayStatics.BreakHitResult` _hitresult))
  (bind _returnvalue (* _distance (`self.Scale`)))
  (bind _returnvalue_2 (`KismetMathLibrary.Normal` (- _tracestart _traceend) 0.1))
  (:`Pressed`
    (if _bblockinghit
      (bind (_species _height _diameter) (`self.Cast2Tree` _hitresult))
      ;[1 1 1] IClicking off a tree closes the box
      (if (`KismetStringLibrary.IsEmpty` _species)
        (set `Widget.Visibility` "Collapsed" (`WidgetComponent.GetWidget` _infocard) :!label _label)
        (`SceneComponent.K2_SetWorldLocationAndRotation` :`self` _infocard)
        (else
          ;[1 1 1] Set Location, Scale, Content, and Make Box Visible
          (bind _astree_info (cast `/Game/Widgets/TreeInfo` (`WidgetComponent.GetWidget` (`self.InfoCard`))))
          (`/Game/Widgets/TreeInfo.SetInfo` _astree_info _species _height _diameter)
          (`SceneComponent.K2_SetWorldLocationAndRotation` _infocard_2 (+ _impactpoint (* (50.0 50.0 50.0) _returnvalue_2)) (`KismetMathLibrary.MakeRotFromX` _returnvalue_2) false false)
          (`SceneComponent.SetWorldScale3D` _infocard_2 (`KismetMathLibrary.MakeVector` (`KismetMathLibrary.FClamp` (.x (* (1.0 1.0 1.0) (`KismetMathLibrary.MakeVector` _returnvalue _returnvalue _returnvalue))) 0.0 2.0) (`KismetMathLibrary.FClamp` (.y (* (1.0 1.0 1.0) (`KismetMathLibrary.MakeVector` _returnvalue _returnvalue _returnvalue))) 0.0 2.0) (`KismetMathLibrary.FClamp` (.z (* (1.0 1.0 1.0) (`KismetMathLibrary.MakeVector` _returnvalue _returnvalue _returnvalue))) 0.0 2.0)))
          (set `Widget.Visibility` "Visible" (`WidgetComponent.GetWidget` _infocard_2))))
      (else
        (goto _label)))))

(event `Key|LeftShift`
  (params (Key :type "Key Structure"))
  (bind _returnvalue (`GameplayStatics.GetPlayerController` 0))
  ;[1 1 1] Show mouse when shift is pressed
  (:`Pressed`
    (set `PlayerController.bShowMouseCursor` true _returnvalue :!label _label_2))
  (:`Released`
    (set `PlayerController.bShowMouseCursor` false _returnvalue :!label _label_3)))

(event `Key|RightShift`
  (params (Key :type "Key Structure"))
  ;[1 1 1] Show mouse when shift is pressed
  (:`Pressed`
    (goto _label_2))
  (:`Released`
    (goto _label_3)))

(fn `Cast2Tree`
  (params (`Hit Result` :type "HitResult Structure"))
  (returns (Species :type String) (Height :type "Float (double-precision)") (Diameter :type "Float (double-precision)"))
  (bind (_bblockinghit _binitialoverlap _time _distance _location _impactpoint _normal _impactnormal _physmat _hitactor _hitcomponent _hitbonename _bonename _hititem) (`GameplayStatics.BreakHitResult` `Hit Result`))
  ;[1 1 1] Cast to Tree Manager Thinning, and Get Info of Clicked on Tree
  (bind _astree_manager_thinning (cast `/Game/Blueprints/TreeManagerThinning` _hitactor)
    (:`then`
      (cast `HierarchicalInstancedStaticMeshComponent` _hitcomponent)
      (bind (_species _height _diameter) (`/Game/Blueprints/TreeManagerThinning.GetInstanceInfo` _astree_manager_thinning _hitcomponent _hititem))
      (return _species _height _diameter))
    (:`CastFailed`
      ;[1 1 1] Cast to Tree Manager, and Get Info of Clicked on Tree
      (bind _astree_manager (cast `/Game/Blueprints/TreeManager` _hitactor)
        (:`then`
          (cast `HierarchicalInstancedStaticMeshComponent` _hitcomponent)
          (bind (_species_2 _height_2 _diameter_2) (`/Game/Blueprints/TreeManager.GetInstanceInfo` _astree_manager _hitcomponent _hititem))
          (return _species_2 _height_2 _diameter_2))
        (:`CastFailed`
          ;[1 1 1] Cast Failed, Species is Empty on Purpose
          (return "" 0.0 0.0))))))

(fn `UserConstructionScript`)